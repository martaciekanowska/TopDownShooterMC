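; BP_Soldier_01 is the player-controlled soldier, with world-axis movement, mouse-steered facing and an assault rifle effect.
; Each tick, mouse velocity above a dead zone is converted by Atan2 into a yaw that the control rotation interpolates toward.
; Fire input toggles the muzzle flash and looping fire sound, with an end sound on release; no projectile or damage logic runs here.
; BeginPlay switches the flash off and adds the player HUD.
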(event `self.ReceiveTick`
  (params (DeltaSeconds :type "Float (single-precision)"))
  ;[0.5121 1 0.3254] Rotation
  (`self.UpdatePlayerRotation`))

(event `InputAxis|MoveForward`
  (params (AxisValue :type "Float (single-precision)"))
  ;[0.3806 0.5073 1] Movement
  (`self.AddMovementInput` (1.0 0.0 0.0) AxisValue))

(event `InputAxis|MoveLeftRight`
  (params (AxisValue :type "Float (single-precision)"))
  ;[0.3806 0.5073 1] Movement
  (`self.AddMovementInput` (0.0 1.0 0.0) AxisValue))

(event `InputAction|FireWeapon`
  (params (Key :type "Key Structure"))
  ;[1 0.3944 0.8908] FX Weapon
  (:`Pressed`
    (`self.StartFiringWeapon`))
  (:`Released`
    (`self.StopFiringWeapon`)))

(event `self.ReceiveBeginPlay`
  (`ActorComponent.Deactivate` (`self.P_AssaultRifle_MF`))
  (bind _returnvalue (`|CreateWidget` "/Game/UI/W_PlayerHUD.W_PlayerHUD_C" null self))
  (`UserWidget.AddToViewport` _returnvalue 0))

(fn `GetMouseVelocity`
  (returns (ReturnValue :type "Vector2D Structure"))
  (bind (_deltax _deltay) (`PlayerController.GetInputMouseDelta` (`GameplayStatics.GetPlayerController` 0)))
  (return (/ (`KismetMathLibrary.MakeVector2D` _deltax _deltay) (`GameplayStatics.GetWorldDeltaSeconds`))))

(fn `IsMouseAboveDeadZone`
  (returns (ReturnValue :type Boolean))
  (return (> (`KismetMathLibrary.VSize2D` (`self.GetMouseVelocity`)) (`self.MouseDeadZone`))))

(fn `StartFiringWeapon`
  (`ActorComponent.Activate` (`self.P_AssaultRifle_MF`) false)
  (bind _returnvalue (`GameplayStatics.SpawnSound2D` "/Game/Sounds/Weapon_AssaultRifle/Stereo/RandomFireloop.RandomFireloop" 1.0 1.0 0.0 null))
  (set `self.Rifle_Firesound` _returnvalue))

(fn `StopFiringWeapon`
  (`ActorComponent.Deactivate` (`self.P_AssaultRifle_MF`))
  (`AudioComponent.Stop` (`self.Rifle_Firesound`))
  (`GameplayStatics.SpawnSound2D` "/Game/Sounds/Weapon_AssaultRifle/Stereo/Assult_Rifle_Endshoot.Assult_Rifle_Endshoot" 1.0 1.0 0.0 null))

(fn `UpdatePlayerRotation`
  (bind (_returnvalue_x _returnvalue_y) (`KismetMathLibrary.BreakVector2D` (`self.GetMouseVelocity`)))
  (bind _returnvalue (`GameplayStatics.GetPlayerController` 0))
  (if (`self.IsMouseAboveDeadZone`)
    (`Controller.SetControlRotation` _returnvalue (`KismetMathLibrary.RInterpTo` (`Controller.GetControlRotation` _returnvalue) (`KismetMathLibrary.MakeRotator` 0.0 0.0 (`KismetMathLibrary.DegAtan2` _returnvalue_x _returnvalue_y)) (`GameplayStatics.GetWorldDeltaSeconds`) (`self.DeltaTimeMultiply`)))))

(fn `UserConstructionScript`)